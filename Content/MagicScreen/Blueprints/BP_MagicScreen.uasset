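; BP_MagicScreen is a video screen that acts as a window through which AR objects are seen, showing textures passed to UpdateVideoFrame.
; Each tick it writes either four planes through the player camera and screen corners, or just the corners, to a parameter collection, letting AR materials hide anything outside that frustum.
; The corners-only mode supports Simulate, where camera position is unavailable.
; A flipped ScreenBack mesh casts the translucent screen's shadow.
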(event EventBeginPlay
  ;[1 1 1] Creating a dynamic instance of our video screen material of choice, and applying it to the screen mesh (a plane)
  (bind _returnvalue (Rendering|Material|CreateDynamicMaterialInstance (Variables|Default|GetScreen) 0 (Variables|Default|GetVideoScreenMaterial) :!class /Script/Engine.PrimitiveComponent))
  (bind _output_get (Variables|Default|SetDynamicMaterial _returnvalue))
  (Rendering|Material|SetMaterial (Variables|Default|GetScreen) 0 _output_get))

(event EventTick
  (params (DeltaSeconds :type Float%20%28single-precision%29))
  ;[1 1 1] This function updates the "frustum" out of which the AR objects should not be seen.
  ; It needs to be done on Tick since it depends on the current camera position.
  (CallFunction|UpdateFrustum))

(fn ConstructionScript
  (CallFunction|UpdateFrustum)
  ;[1 1 1] We need this, since the screen is translucent and won't cast shadows
  (CallFunction|SetupScreenShadowObject))

(fn UpdateCorners
  (Utilities|FlowControl|Sequence
    (:then_0
      ;[1 1 1] Storing corners locations inside a material parameters collection, accessible by the AR objects materials
      (Rendering|Material|SetVectorParameterValue "/MagicUtilities/MagicScreen/Materials/MagicSCreenCameraParametersCollection.MagicScreenCameraParametersCollection" "CornerA" (Math|Conversions|ToLinearColor(Vector) (Transformation|GetWorldLocation (Variables|Default|GetCorner_A))) :!class /Script/Engine.KismetMaterialLibrary))
    (:then_1
      (Rendering|Material|SetVectorParameterValue "/MagicUtilities/MagicScreen/Materials/MagicSCreenCameraParametersCollection.MagicScreenCameraParametersCollection" "CornerB" (Math|Conversions|ToLinearColor(Vector) (Transformation|GetWorldLocation (Variables|Default|GetCorner_B))) :!class /Script/Engine.KismetMaterialLibrary))
    (:then_2
      (Rendering|Material|SetVectorParameterValue "/MagicUtilities/MagicScreen/Materials/MagicSCreenCameraParametersCollection.MagicScreenCameraParametersCollection" "CornerC" (Math|Conversions|ToLinearColor(Vector) (Transformation|GetWorldLocation (Variables|Default|GetCorner_C))) :!class /Script/Engine.KismetMaterialLibrary))
    (:then_3
      (Rendering|Material|SetVectorParameterValue "/MagicUtilities/MagicScreen/Materials/MagicSCreenCameraParametersCollection.MagicScreenCameraParametersCollection" "CornerD" (Math|Conversions|ToLinearColor(Vector) (Transformation|GetWorldLocation (Variables|Default|GetCorner_D))) :!class /Script/Engine.KismetMaterialLibrary))))

(fn UpdateFrustumPlanesCoefficients
  (Utilities|FlowControl|Sequence
    (:then_0
      ;[1 1 1] Retrieve screen corners and player camera location
      (LocalVariables|SetCornerA (Transformation|GetWorldLocation (Variables|Default|GetCorner_A))))
    (:then_1
      (LocalVariables|SetCornerB (Transformation|GetWorldLocation (Variables|Default|GetCorner_B))))
    (:then_2
      (LocalVariables|SetCornerC (Transformation|GetWorldLocation (Variables|Default|GetCorner_C))))
    (:then_3
      (LocalVariables|SetCornerD (Transformation|GetWorldLocation (Variables|Default|GetCorner_D))))
    (:then_4
      (LocalVariables|SetCameraLocation (Camera|GetCameraLocation (Game|GetPlayerCameraManager 0))))
    (:then_5
      (Utilities|FlowControl|Sequence
        (:then_0
          ;[1 1 1] computing a, b, c, d coefficients for the 4 planes needed to define our rough frustum,
          ; and storing them locations inside a material parameters collection, accessible by the AR objects materials
          (Rendering|Material|SetVectorParameterValue "/MagicUtilities/MagicScreen/Materials/MagicSCreenCameraParametersCollection.MagicScreenCameraParametersCollection" "PlaneUp" (Utilities|Struct|MakeLinearColor (.x (Class|GeometryUtilities|MakePlanefromThreePoints (LocalVariables|GetCameraLocation) (LocalVariables|GetCornerA) (LocalVariables|GetCornerB))) (.y (Class|GeometryUtilities|MakePlanefromThreePoints (LocalVariables|GetCameraLocation) (LocalVariables|GetCornerA) (LocalVariables|GetCornerB))) (.z (Class|GeometryUtilities|MakePlanefromThreePoints (LocalVariables|GetCameraLocation) (LocalVariables|GetCornerA) (LocalVariables|GetCornerB))) (.w (Class|GeometryUtilities|MakePlanefromThreePoints (LocalVariables|GetCameraLocation) (LocalVariables|GetCornerA) (LocalVariables|GetCornerB)))) :!class /Script/Engine.KismetMaterialLibrary))
        (:then_1
          (Rendering|Material|SetVectorParameterValue "/MagicUtilities/MagicScreen/Materials/MagicSCreenCameraParametersCollection.MagicScreenCameraParametersCollection" "PlaneLeft" (Utilities|Struct|MakeLinearColor (.x (Class|GeometryUtilities|MakePlanefromThreePoints (LocalVariables|GetCameraLocation) (LocalVariables|GetCornerA) (LocalVariables|GetCornerD))) (.y (Class|GeometryUtilities|MakePlanefromThreePoints (LocalVariables|GetCameraLocation) (LocalVariables|GetCornerA) (LocalVariables|GetCornerD))) (.z (Class|GeometryUtilities|MakePlanefromThreePoints (LocalVariables|GetCameraLocation) (LocalVariables|GetCornerA) (LocalVariables|GetCornerD))) (.w (Class|GeometryUtilities|MakePlanefromThreePoints (LocalVariables|GetCameraLocation) (LocalVariables|GetCornerA) (LocalVariables|GetCornerD)))) :!class /Script/Engine.KismetMaterialLibrary))
        (:then_2
          (Rendering|Material|SetVectorParameterValue "/MagicUtilities/MagicScreen/Materials/MagicSCreenCameraParametersCollection.MagicScreenCameraParametersCollection" "PlaneRight" (Utilities|Struct|MakeLinearColor (.x (Class|GeometryUtilities|MakePlanefromThreePoints (LocalVariables|GetCameraLocation) (LocalVariables|GetCornerB) (LocalVariables|GetCornerC))) (.y (Class|GeometryUtilities|MakePlanefromThreePoints (LocalVariables|GetCameraLocation) (LocalVariables|GetCornerB) (LocalVariables|GetCornerC))) (.z (Class|GeometryUtilities|MakePlanefromThreePoints (LocalVariables|GetCameraLocation) (LocalVariables|GetCornerB) (LocalVariables|GetCornerC))) (.w (Class|GeometryUtilities|MakePlanefromThreePoints (LocalVariables|GetCameraLocation) (LocalVariables|GetCornerB) (LocalVariables|GetCornerC)))) :!class /Script/Engine.KismetMaterialLibrary))
        (:then_3
          (Rendering|Material|SetVectorParameterValue "/MagicUtilities/MagicScreen/Materials/MagicSCreenCameraParametersCollection.MagicScreenCameraParametersCollection" "PlaneBottom" (Utilities|Struct|MakeLinearColor (.x (Class|GeometryUtilities|MakePlanefromThreePoints (LocalVariables|GetCameraLocation) (LocalVariables|GetCornerC) (LocalVariables|GetCornerD))) (.y (Class|GeometryUtilities|MakePlanefromThreePoints (LocalVariables|GetCameraLocation) (LocalVariables|GetCornerC) (LocalVariables|GetCornerD))) (.z (Class|GeometryUtilities|MakePlanefromThreePoints (LocalVariables|GetCameraLocation) (LocalVariables|GetCornerC) (LocalVariables|GetCornerD))) (.w (Class|GeometryUtilities|MakePlanefromThreePoints (LocalVariables|GetCameraLocation) (LocalVariables|GetCornerC) (LocalVariables|GetCornerD)))) :!class /Script/Engine.KismetMaterialLibrary))))))

(fn UpdateFrustum
  (if (Variables|Settings|GetUsingOptimizedARObjectsMaterial)
    ;[1 1 1] This function updates the "frustum" out of which the AR objects should not be seen.
    ; It needs to be done on Tick since it depends on the current camera position.
    (CallFunction|UpdateFrustumPlanesCoefficients)
    (else
      ;[1 1 1] The frustum update function doesn't work with simulation mode, since the camera position is unavailable.
      ;
      ; To overcome this limitation, the frustum is computed directly inside each AR object material.
      ;
      ; This is not optimal, but useful during development
      (CallFunction|UpdateCorners))))

(fn UpdateVideoFrame
  (params (FrameTexture :type Texture%20Object%20Reference))
  ;[1 1 1] Update the screen content with a new texture
  (Rendering|Material|SetTextureParameterValue (Variables|Default|GetDynamicMaterial) "Texture" FrameTexture))

(fn SetupScreenShadowObject
  (bind _screen (Variables|Default|GetScreen))
  (bind _returnvalue (Transformation|GetWorldTransform _screen))
  (Components|StaticMesh|SetStaticMesh (Variables|Default|GetScreenBack) (Variables|/Script/Engine.StaticMeshComponent|GetStaticMesh (Variables|Default|GetScreen)))
  (Rendering|SetCastShadow (Variables|Default|GetScreenBack) true)
  (Rendering|SetVisibility (Variables|Default|GetScreenBack) true false)
  (Class|PrimitiveComponent|SetRenderinMainPass (Variables|Default|GetScreenBack) true)
  (Transformation|SetWorldTransform (Variables|Default|GetScreenBack) (Math|Transform|MakeTransform (.location _returnvalue) (Math|Rotator|CombineRotators (.rotation _returnvalue) "180.000000, 0, 0") (.scale _returnvalue)) false false))