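; Static mesh actor for the magic screen feature, using a dynamic material with its "DrawAnyway" parameter forced off.
; The construction script creates that material instance from ObjectMaterial if none exists and applies it to the mesh.
; CheckIfDrawAnyway zeroes the parameter at construction and BeginPlay, with no actual condition.
; ShadowMesh copies the same mesh as a shadow proxy, casting shadows while excluded from the main render pass.
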(event EventBeginPlay
  (CallFunction|CheckifDrawAnyway))

(fn ConstructionScript
  (Utilities|FlowControl|Sequence
    (:then_0
      (Utilities|IsValid (Variables|Appearance|GetDynamicMaterialInstance)
        (:Is%20Not%20Valid
          (bind _returnvalue (Rendering|Material|CreateDynamicMaterialInstance (Variables|Debug|GetStaticMeshComponent) 0 (Variables|Appearance|GetObjectMaterial) :!class /Script/Engine.PrimitiveComponent))
          (bind _output_get (Variables|Appearance|SetDynamicMaterialInstance _returnvalue))
          (Rendering|Material|SetMaterial (Variables|Debug|GetStaticMeshComponent) 0 _output_get))))
    (:then_1
      (CallFunction|CheckifDrawAnyway)
      (Components|StaticMesh|SetStaticMesh (Variables|Default|GetShadowMesh) (Variables|/Script/Engine.StaticMeshComponent|GetStaticMesh (Variables|Debug|GetStaticMeshComponent)))
      (Rendering|SetCastShadow (Variables|Default|GetShadowMesh) true)
      (Rendering|SetVisibility (Variables|Default|GetShadowMesh) true false)
      (Class|PrimitiveComponent|SetRenderinMainPass (Variables|Default|GetShadowMesh) false))))

(fn CheckifDrawAnyway
  (Rendering|Material|SetScalarParameterValue (Variables|Appearance|GetDynamicMaterialInstance) "DrawAnyway" 0.0 :!class /Script/Engine.MaterialInstanceDynamic))