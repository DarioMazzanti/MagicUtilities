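; Static mesh actor for the MagicScreen feature that toggles a "DrawAnyway" override on its material.
; The construction script creates a dynamic instance of ObjectMaterial on slot 0 if none exists, then writes the DrawAnyway flag to it as a 0/1 scalar parameter.
; BeginPlay forces the flag off and reapplies it, so the override only has an effect outside of play, such as in editor preview.
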(event EventBeginPlay
  (Variables|Appearance|SetDrawAnyway false)
  (CallFunction|CheckifDrawAnyway))

(fn ConstructionScript
  (Utilities|FlowControl|Sequence
    (:then_0
      (Utilities|IsValid (Variables|Appearance|GetDynamicMaterialInstance)
        (:Is%20Not%20Valid
          (bind _returnvalue (Rendering|Material|CreateDynamicMaterialInstance (Variables|Debug|GetStaticMeshComponent) 0 (Variables|Appearance|GetObjectMaterial) :!class /Script/Engine.PrimitiveComponent))
          (bind _output_get (Variables|Appearance|SetDynamicMaterialInstance _returnvalue))
          (Rendering|Material|SetMaterial (Variables|Debug|GetStaticMeshComponent) 0 _output_get))))
    (:then_1
      (CallFunction|CheckifDrawAnyway))))

(fn CheckifDrawAnyway
  (if (Variables|Appearance|GetDrawAnyway)
    (Rendering|Material|SetScalarParameterValue (Variables|Appearance|GetDynamicMaterialInstance) "DrawAnyway" 1.0 :!class /Script/Engine.MaterialInstanceDynamic)
    (else
      (Rendering|Material|SetScalarParameterValue (Variables|Appearance|GetDynamicMaterialInstance) "DrawAnyway" 0.0 :!class /Script/Engine.MaterialInstanceDynamic))))